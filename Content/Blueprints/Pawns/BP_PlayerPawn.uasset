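; Player pawn for a rolling-ball game, moved by applying torque to the ball from forward and sideways axis input, scaled by Speed.
; Any damage plays a lose sound and runs the Restartlevel macro once, which fades to black and reopens the current level.
; BeginPlay fades in from black, and AdjustSpringArm sets camera boom length and world rotation.
; Ball resizing is unfinished and unconnected.
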(event `self.ReceiveAnyDamage`
  (params (Damage :type "Float (single-precision)") (DamageType :type "DamageType Object Reference") (InstigatedBy :type "Controller Object Reference") (DamageCauser :type "Actor Object Reference"))
  ;[1 1 1] If Damaged reset current level via Restart Level macro
  (`/Engine/EditorBlueprintResources/StandardMacros.DoOnce` false
    (:`Completed`
      (`GameplayStatics.PlaySound2D` "/Game/Audio/Win-Lose/Lose.Lose" 1.0 1.0 0.0 null null)
      (`self.restartlevel`))))

(event `self.ReceiveBeginPlay`
  ;[1 1 1] Camera Fade in on level start/reset
  (`PlayerCameraManager.StartCameraFade` (`GameplayStatics.GetPlayerCameraManager` 0) 1.0 0.0 3.0 (struct :`A` 1.0) true true))

(event `InputAxis|Move Forwards/Backwards`
  (params (AxisValue :type "Float (single-precision)"))
  ;[1 1 1] Apply Torque for movement and set speed
  (`PrimitiveComponent.AddTorqueInRadians` (`self.Ball`) (`KismetMathLibrary.MakeVector` (* AxisValue (`self.Speed`))) "None" true))

(event `InputAxis|Move Right/Left`
  (params (AxisValue :type "Float (single-precision)"))
  ;[1 1 1] Apply Torque for movement and set speed
  (`PrimitiveComponent.AddTorqueInRadians` (`self.Ball`) (`KismetMathLibrary.MakeVector` 0.0 (* (`self.Speed`) AxisValue)) "None" true))

(fn `AdjustSpringArm`
  (params (Distance :type "Float (double-precision)") (Roll :type "Float (double-precision)") (Pitch :type "Float (double-precision)") (Yaw :type "Float (double-precision)"))
  (bind _springarm (`self.SpringArm`))
  (set `SpringArmComponent.TargetArmLength` Distance _springarm)
  (`SceneComponent.K2_SetWorldRotation` _springarm (`KismetMathLibrary.MakeRotator` Roll Pitch Yaw) false false))

(fn `UserConstructionScript`)