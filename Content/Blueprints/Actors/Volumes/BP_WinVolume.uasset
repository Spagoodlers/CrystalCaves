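; Level-exit trigger volume that runs level completion when the player overlaps its box while BP_Crystal actors remain.
; CompleteLevel rechecks for crystals, opening Level1 if any remain and otherwise the next entry in LevelNames after the current level.
; As wired, the overlap only reaches the Level1 branch, because both checks require remaining crystals.
; IsFinalLevel is defined but never called here.
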(event `self.Box.OnComponentBeginOverlap`
  (params (OverlappedComponent :type "PrimitiveComponent Object Reference") (OtherActor :type "Actor Object Reference") (OtherComp :type "PrimitiveComponent Object Reference") (OtherBodyIndex :type Integer) (bFromSweep :type Boolean) (SweepResult :type "HitResult Structure (by ref)"))
  (`/Game/Blueprints/Libraries/CC_MacroLibrary.IsPlayer` OtherActor
    (:`IsPlayer`
      (if (`self.AnyCrystalsRemaining`)
        (`self.CompleteLevel`)))))

(fn `AnyCrystalsRemaining`
  (returns (CrystalsRemaining :type Boolean))
  (bind _outactors (`GameplayStatics.GetAllActorsOfClass` "/Game/Blueprints/Actors/Collectables/BP_Crystal.BP_Crystal_C"))
  (return (> (`KismetArrayLibrary.Array_Length` _outactors) 0)))

(fn `CompleteLevel`
  (if (`self.AnyCrystalsRemaining`)
    (`GameplayStatics.OpenLevel` "Level1")
    (else
      (`self.LoadNextLevel`))))

(fn `GetCurrentLevelIndex`
  (returns (CurrentLevelIndex :type Integer))
  (bind _returnvalue (`GameplayStatics.GetCurrentLevelName` true))
  (return (`KismetArrayLibrary.Array_Find` (`self.LevelNames`) (`KismetStringLibrary.Conv_StringToName` _returnvalue))))

(fn `GetNextLevelName`
  (returns (ReturnValue :type Name))
  (return (`|GetArrayItem` (`self.LevelNames`) (+ (`self.GetCurrentLevelIndex`) 1))))

(fn `IsFinalLevel`
  (returns (Return :type Boolean))
  (return (== (`KismetArrayLibrary.Array_LastIndex` (`self.LevelNames`)) (`self.GetCurrentLevelIndex`))))

(fn `LoadNextLevel`
  (returns (NextLeveltoLoad :type Name))
  (`GameplayStatics.OpenLevel` (`self.GetNextLevelName`)))

(fn `UserConstructionScript`)