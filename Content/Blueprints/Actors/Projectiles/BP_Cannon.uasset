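; BP_Cannon is an automatic cannon actor that repeatedly fires BP_Projectile from its spawn point.
; BeginPlay starts a loop that waits for the fire rate, spawns a scaled projectile, plays the cannon sound and starts a Timeline.
; The Timeline slides the barrel along its local Y axis, and its Cannon Fired event track restarts the loop, so the animation also paces the shots.
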(event `self.ReceiveBeginPlay`
  (`KismetSystemLibrary.Delay` (`self.FireRate`) :!label _label)
  (`self.Spawn Projectile`)
  (`GameplayStatics.PlaySoundAtLocation` "/Game/Audio/Weapons/Cannon/cannon.cannon" (0.0 0.0 0.0) (struct) 0.1 -1.0 0.0 null null null)
  (bind (_direction _cannonbarrelllocation) (`Timeline|CannonFireAnimation` :!via `PlayFromStart`)
    (:`Update`
      (`self.MoveBarrell` _cannonbarrelllocation))
    (:`CannonFired`
      (goto _label))))

(fn `MoveBarrell`
  (params (`Cannon Barrell Y Location` :type "Float (double-precision)"))
  (`SceneComponent.K2_SetRelativeLocation` (`self.barrel`) (`KismetMathLibrary.MakeVector` 0.0 `Cannon Barrell Y Location`) false false))

(fn `Spawn Projectile`
  (bind _projectilespawn (`self.projectilespawn`))
  (`|SpawnActorFromClass` "/Game/Blueprints/Actors/Projectiles/BP_Projectile.BP_Projectile_C" (`KismetMathLibrary.MakeTransform` (`SceneComponent.K2_GetComponentLocation` _projectilespawn) (`SceneComponent.K2_GetComponentRotation` _projectilespawn) (`KismetMathLibrary.Conv_DoubleToVector` (`self.ProjectileScale`))) "Undefined" "OverrideRootScale" null null))

(fn `UserConstructionScript`)