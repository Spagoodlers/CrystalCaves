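; BP_Crystal is a collectable crystal that the player picks up by overlapping it.
; On player overlap it stores its location and scale, then plays CollectionTimeline.
; Each timeline update lerps the crystal toward the player's current position, shrinks it toward zero and fades CrystalLight, with a DoOnce playing the pickup sound a single time.
; The actor destroys itself when the timeline finishes.
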(event `self.ReceiveActorBeginOverlap`
  (params (OtherActor :type "Actor Object Reference"))
  (`/Game/Blueprints/Libraries/CC_MacroLibrary.IsPlayer` OtherActor
    (:`IsPlayer`
      (`self.StoreStartingValues`)
      (bind (_direction _collectionprogress _scaleprogress _light_intensity) (`Timeline|CollectionTimeline`)
        (:`Update`
          (`self.MoveToPlayer` _collectionprogress)
          (`self.ScaleCrystal` _scaleprogress)
          (`self.AdjustLight` _light_intensity)
          (`/Engine/EditorBlueprintResources/StandardMacros.DoOnce` false
            (:`Completed`
              (`GameplayStatics.PlaySound2D` "/Game/Audio/CrystalGet.CrystalGet" 1.0 1.0 0.0 null null))))
        (:`Finished`
          (`self.K2_DestroyActor`))))))

(fn `AdjustLight`
  (params (Alpha :type "Float (double-precision)"))
  (`LightComponent.SetIntensity` (`self.Crystal Light`) (`KismetMathLibrary.Lerp` (`self.LightIntensity`) 0.0 Alpha)))

(fn `MoveToPlayer`
  (params (Alpha :type "Float (double-precision)"))
  (`self.K2_SetActorLocation` (`KismetMathLibrary.VLerp` (`self.StartLocation`) (`self.K2_GetActorLocation` (`GameplayStatics.GetPlayerPawn` 0)) Alpha)))

(fn `ScaleCrystal`
  (params (Alpha :type "Float (double-precision)"))
  (`self.SetActorScale3D` (`KismetMathLibrary.VLerp` (`self.StartScale`) (0.0 0.0 0.0) Alpha)))

(fn `StoreStartingValues`
  (set `self.StartLocation` (`self.K2_GetActorLocation`))
  (set `self.StartScale` (`self.GetActorScale3D`)))

(fn `UserConstructionScript`)