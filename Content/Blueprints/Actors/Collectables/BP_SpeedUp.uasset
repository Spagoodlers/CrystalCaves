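; Speed power-up crystal that sets the player pawn's Speed to a boosted value when the player overlaps it.
; A collection timeline pulls the crystal toward the player while shrinking it and fading its light, then destroys the actor when finished.
; On the first timeline update it plays a whoosh and starts a delayed speed reset, which depends on the actor still existing when the delay ends.
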(event `self.ReceiveActorBeginOverlap`
  (params (OtherActor :type "Actor Object Reference"))
  (`self.IsPlayer` OtherActor
    (:`IsPlayer`
      (`self.Change Speedx2`)
      (`self.StoreStartingValues`)
      (bind (_direction _collectionprogress _scaleprogress _light_intensity) (`Timeline|CollectionTimeline`)
        (:`Update`
          (`self.MoveToPlayer` _collectionprogress)
          (`self.ScaleCrystal` _scaleprogress)
          (`self.AdjustLight` _light_intensity)
          (`/Engine/EditorBlueprintResources/StandardMacros.DoOnce` false
            (:`Completed`
              (`GameplayStatics.PlaySound2D` "/Game/Audio/Powerup/speed_whoosh_HbT59u7FDI.speed_whoosh_HbT59u7FDI" 1.0 1.0 0.0 null null)
              (`KismetSystemLibrary.Delay` 8.0)
              (`self.Change Speed/2`))))
        (:`Finished`
          (`self.K2_DestroyActor`))))))

(fn `AdjustLight`
  (params (Alpha :type "Float (double-precision)"))
  (`LightComponent.SetIntensity` (`self.Crystal Light`) (`KismetMathLibrary.Lerp` (`self.LightIntensity`) 0.0 Alpha)))

(fn `Change Speed/2`
  (bind _asbp_player_pawn (cast `/Game/Blueprints/Pawns/BP_PlayerPawn` (`GameplayStatics.GetPlayerPawn` 0)))
  (set `/Game/Blueprints/Pawns/BP_PlayerPawn.Speed` 15.0 _asbp_player_pawn))

(fn `Change Speedx2`
  (bind _asbp_player_pawn (cast `/Game/Blueprints/Pawns/BP_PlayerPawn` (`GameplayStatics.GetPlayerPawn` 0)))
  (set `/Game/Blueprints/Pawns/BP_PlayerPawn.Speed` 30.0 _asbp_player_pawn))

(fn `MoveToPlayer`
  (params (Alpha :type "Float (double-precision)"))
  (`self.K2_SetActorLocation` (`KismetMathLibrary.VLerp` (`self.StartLocation`) (`self.K2_GetActorLocation` (`GameplayStatics.GetPlayerPawn` 0)) Alpha)))

(fn `ScaleCrystal`
  (params (Alpha :type "Float (double-precision)"))
  (`self.SetActorScale3D` (`KismetMathLibrary.VLerp` (`self.StartScale`) (0.0 0.0 0.0) Alpha)))

(fn `StoreStartingValues`
  (set `self.StartLocation` (`self.K2_GetActorLocation`))
  (set `self.StartScale` (`self.GetActorScale3D`)))

(fn `UserConstructionScript`)